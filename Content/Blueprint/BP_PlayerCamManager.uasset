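; Player camera manager that blends the view between the player's normal camera and aim-down-sights on the gun.
; BeginPlay caches the possessed Bp_Player, whose AimAlpha drives location and FOV blends in BlueprintUpdateCamera, while rotation follows control rotation.
; The aimed location is the gun's ADSCam socket, offset along its forward axis by a dot-product projection of the camera-to-socket offset.
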(event `self.ReceiveBeginPlay`
  (bind _asbp_player (cast `/Game/Blueprint/Player/Bp_Player` (`Controller.K2_GetPawn` (`self.GetOwningPlayerController`))))
  (bind _output_get (set `self.PlayerRef` _asbp_player))
  (set `self.DefaultFOV` (`/Game/Blueprint/Player/Bp_Player.NormalFOV` _output_get)))

(fn `BlueprintUpdateCamera`
  (params (CameraTarget :type "Actor Object Reference"))
  (returns (NewCameraLocation :type "Vector Structure") (NewCameraRotation :type "Rotator Structure") (NewCameraFOV :type "Float (double-precision)") (ReturnValue :type Boolean))
  (locals (FinalCamLoc :type "Vector Structure") (FinalCamRot :type "Rotator Structure"))
  (bind _playerref (`self.PlayerRef`))
  (bind _aimalpha (`/Game/Blueprint/Player/Bp_Player.AimAlpha` _playerref))
  (bind _returnvalue (`SceneComponent.K2_GetComponentLocation` (`/Game/Blueprint/Player/Bp_Player.Normal Camera` _playerref)))
  (bind (_returnvalue_location _returnvalue_rotation) (`KismetMathLibrary.BreakTransform` (`SceneComponent.GetSocketTransform` (`/Game/Blueprint/Weapon/GunBase.GunMesh` (`/Game/Blueprint/Player/Bp_Player.GunRef` _playerref)) "ADSCam" "RTS_World")))
  (bind _returnvalue_2 (`KismetMathLibrary.GetForwardVector` _returnvalue_rotation))
  (bind _returnvalue_3 (- _returnvalue _returnvalue_location))
  (if (and (== CameraTarget _playerref) (`KismetSystemLibrary.IsValid` _playerref))
    (set `local.FinalCamRot` (`Pawn.GetControlRotation` _playerref))
    (set `local.FinalCamLoc` (`KismetMathLibrary.VLerp` _returnvalue (- _returnvalue_location (* _returnvalue_2 (* (`KismetMathLibrary.Dot_VectorVector` (`KismetMathLibrary.Normal` _returnvalue_3) _returnvalue_2) (`KismetMathLibrary.VSize` _returnvalue_3)))) _aimalpha))
    (return (`local.FinalCamLoc`) (`local.FinalCamRot`) (`KismetMathLibrary.Lerp` (`/Game/Blueprint/Player/Bp_Player.NormalFOV` _playerref) (`/Game/Blueprint/Player/Bp_Player.ADSFOV` _playerref) _aimalpha) true)))

(fn `UserConstructionScript`)