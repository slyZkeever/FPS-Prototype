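; Ammo pickup actor that refills the player's ammo when the player walks into its box trigger.
; On BeginPlay it caches the player character as Bp_Player.
; On overlap with that player, if ammo is not already full, it adds a fixed amount through UpdateAmmo and plays a pickup sound at its location.
; The pickup is never destroyed or disabled, and a random-amount node is left unconnected.
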(event `self.ReceiveBeginPlay`
  (bind _asbp_player (cast `/Game/Blueprint/Player/Bp_Player` (`GameplayStatics.GetPlayerCharacter` 0)))
  (set `self.PlayerRef` _asbp_player))

(event `self.Box.OnComponentBeginOverlap`
  (params (OverlappedComponent :type "PrimitiveComponent Object Reference") (OtherActor :type "Actor Object Reference") (OtherComp :type "PrimitiveComponent Object Reference") (OtherBodyIndex :type Integer) (bFromSweep :type Boolean) (SweepResult :type "HitResult Structure (by ref)"))
  (bind _playerref (`self.PlayerRef`))
  (if (== OtherActor (`self.PlayerRef`))
    (bind _value (`/Game/Blueprint/Player/Bp_Player.HasFullAmmo` _playerref))
    (if (not _value)
      (`/Game/Blueprint/Player/Bp_Player.UpdateAmmo` _playerref 120)
      (`GameplayStatics.PlaySoundAtLocation` "/Game/Sounds/Weapon_AssaultRifle/Mono/AssaultRifle_AmmoPickup_Cue.AssaultRifle_AmmoPickup_Cue" (`self.K2_GetActorLocation`) (struct) 1.0 1.0 0.0 null null null))))

(fn `UserConstructionScript`)