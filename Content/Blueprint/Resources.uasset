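; Resources is a pickup actor that restores health and ammo to the player when they overlap its Box.
; It caches the player's Bp_Player on BeginPlay and ignores overlaps from any other actor.
; Health and ammo are checked independently, each receiving a random amount within configurable bounds and a pickup sound only when below full.
; The graph never destroys or disables the actor, so every new overlap can grant again.
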(event `self.ReceiveBeginPlay`
  (bind _asbp_player (cast `/Game/Blueprint/Player/Bp_Player` (`GameplayStatics.GetPlayerCharacter` 0)))
  (set `self.PlayerRef` _asbp_player))

(event `self.Box.OnComponentBeginOverlap`
  (params (OverlappedComponent :type "PrimitiveComponent Object Reference") (OtherActor :type "Actor Object Reference") (OtherComp :type "PrimitiveComponent Object Reference") (OtherBodyIndex :type Integer) (bFromSweep :type Boolean) (SweepResult :type "HitResult Structure (by ref)"))
  (bind _returnvalue (`self.K2_GetActorLocation`))
  (bind _playerref (`self.PlayerRef`))
  (if (== OtherActor (`self.PlayerRef`))
    (`|ExecutionSequence`
      (:`then_0`
        (if (< (`/Game/Blueprint/Player/Bp_Player.Health` (`self.PlayerRef`)) 100.0)
          (`/Game/Blueprint/Player/Bp_Player.UpdateHealth` (`self.PlayerRef`) (`KismetMathLibrary.RandomFloatInRange` (`self.MinHealthAdditive`) (`self.MaxHealthAdditive`)))
          (`GameplayStatics.PlaySoundAtLocation` "/Game/Sounds/Stingers/Mono/StingerPickup_Health_Cue.StingerPickup_Health_Cue" _returnvalue (struct) 1.0 1.0 0.0 null null null)))
      (:`then_1`
        (bind _value (`/Game/Blueprint/Player/Bp_Player.HasFullAmmo` _playerref))
        (if (not _value)
          (`/Game/Blueprint/Player/Bp_Player.UpdateAmmo` _playerref (`KismetMathLibrary.RandomIntegerInRange` (`self.MinAmmoAdditive`) (`self.MaxAmmoAdditive`)))
          (`GameplayStatics.PlaySoundAtLocation` "/Game/Sounds/Weapon_AssaultRifle/Mono/AssaultRifle_AmmoPickup_Cue.AssaultRifle_AmmoPickup_Cue" _returnvalue (struct) 1.0 1.0 0.0 null null null))))))

(fn `UserConstructionScript`)