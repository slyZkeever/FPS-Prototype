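; Health pickup actor that restores a random amount of health to the player on overlap.
; BeginPlay caches the player character as Bp_Player, and the Box overlap responds only to that actor while its Health is below 100.
; It passes a random value between MinHealthAdditive and MaxHealthAdditive to UpdateHealth, then plays a pickup sound at its location.
; The graph never destroys or disables the pickup after use.
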(event `self.ReceiveBeginPlay`
  (bind _asbp_player (cast `/Game/Blueprint/Player/Bp_Player` (`GameplayStatics.GetPlayerCharacter` 0)))
  (set `self.PlayerRef` _asbp_player))

(event `self.Box.OnComponentBeginOverlap`
  (params (OverlappedComponent :type "PrimitiveComponent Object Reference") (OtherActor :type "Actor Object Reference") (OtherComp :type "PrimitiveComponent Object Reference") (OtherBodyIndex :type Integer) (bFromSweep :type Boolean) (SweepResult :type "HitResult Structure (by ref)"))
  (if (== OtherActor (`self.PlayerRef`))
    (if (< (`/Game/Blueprint/Player/Bp_Player.Health` (`self.PlayerRef`)) 100.0)
      (`/Game/Blueprint/Player/Bp_Player.UpdateHealth` (`self.PlayerRef`) (`KismetMathLibrary.RandomFloatInRange` (`self.MinHealthAdditive`) (`self.MaxHealthAdditive`)))
      (`GameplayStatics.PlaySoundAtLocation` "/Game/Sounds/Stingers/Mono/StingerPickup_Health_Cue.StingerPickup_Health_Cue" (`self.K2_GetActorLocation`) (struct) 1.0 1.0 0.0 null null null))))

(fn `UserConstructionScript`)